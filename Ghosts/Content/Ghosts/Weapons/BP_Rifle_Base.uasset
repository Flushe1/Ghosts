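; Base rifle Blueprint that responds to GhostsFirearm fire, dry-fire and reload events.
; Firing with ammo runs a debug-drawn hitscan Visibility trace from the player camera, applying fixed damage on a hit.
; Both shot and impact sounds play only when the trace hits.
; Reload start plays a sound, while dry fire, reload states and hit actor names use debug prints.
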(event OnFired(GhostsFirearm)
  (bind _returnvalue (Game|GetPlayerCameraManager 0))
  (bind _returnvalue_2 (Camera|GetCameraLocation _returnvalue))
  (if (> (Variables|Default|GetCurrentAmmo) 0)
    (bind (_outhit _returnvalue_3) (Collision|LineTraceByChannel _returnvalue_2 (+ _returnvalue_2 (* (Math|Vector|GetForwardVector (Camera|GetCameraRotation _returnvalue)) "10000.000000,10000.000000,10000.000000")) "TraceTypeQuery1" false 0 "ForDuration"))
    (if _returnvalue_3
      (Development|PrintString (Utilities|GetDisplayName (.HitActor (Collision|BreakHitResult _outhit))))
      (Game|Damage|ApplyDamage (.HitActor (Collision|BreakHitResult _outhit)) 25.0 0 0)
      (Audio|PlaySoundatLocation "/Game/Audio/Weapon_Audio/SW_RifleShot.SW_RifleShot" (Transformation|GetActorLocation) "0, 0, 0" 1.0 1.0 0.0 0 0 0 0)
      (Audio|PlaySoundatLocation "/Game/Audio/Weapon_Audio/SW_BulletImpact.SW_BulletImpact" (.ImpactPoint (Collision|BreakHitResult _outhit)) "0, 0, 0" 1.0 1.0 0.0 0 0 0 0))))

(event OnDryFired(GhostsFirearm)
  (Development|PrintString "CLICK"))

(event OnReloadStarted(GhostsFirearm)
  (Development|PrintString "REALODING")
  (Audio|PlaySoundatLocation "/Game/Audio/Weapon_Audio/SW_Reload.SW_Reload" (Transformation|GetActorLocation) "0, 0, 0" 1.0 1.0 0.0 0 0 0 0))

(event OnReloadFinished(GhostsFirearm)
  (Development|PrintString "RELOADED"))

(fn ConstructionScript)